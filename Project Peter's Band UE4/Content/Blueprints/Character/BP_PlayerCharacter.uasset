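; Player character Blueprint that restores its checkpoint position from the PlayerSaveGame slot.
; On BeginPlay it loads and caches the TheSaveGame object, and if the IsStarting flag is set, teleports to the saved checkpoint and clears the flag.
; On EndPlay it writes the cached save object back to the slot.
; It creates no save object, so a failed load or cast skips the restore.
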(event EventEndPlay
  (params (EndPlayReason :type EEndPlayReason%20Enum :default "Destroyed"))
  (SaveGame|SaveGametoSlot (Variables|Default|GetSaveGameInstance) "PlayerSaveGame"))

(event EventBeginPlay
  (bind _returnvalue (SaveGame|LoadGamefromSlot "PlayerSaveGame"))
  (bind _asthe_save_game (Utilities|Casting|CastToTheSaveGame _returnvalue))
  (bind _output_get (Variables|Default|SetSaveGameInstance _asthe_save_game))
  (bind _returnvalue_2 (Class|TheSaveGame|GetIsStarting _asthe_save_game))
  (if _returnvalue_2
    (bind _returnvalue_3 (Class|TheSaveGame|ReturnCheckPoint _asthe_save_game))
    (Transformation|SetActorLocation _returnvalue_3 false true)
    (Class|TheSaveGame|SetIsStarting _output_get false)))

(fn ConstructionScript)