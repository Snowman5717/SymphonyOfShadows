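; Player HUD Blueprint that draws a subtitle string on screen below the vertical center, offset in from the left edge.
; DrawHUD renders Subtitles each frame with configurable font, color and scale while a short fixed Delay runs.
; When the Delay completes it sets TextDisplayed, so a following frame clears the text and resets the flag.
; The Delay cycles continuously rather than starting when Subtitles changes.
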(event EventDrawHUD
  (params (SizeX :type Integer) (SizeY :type Integer))
  (Variables|Default|SetDelayTimer 3.0)
  (if (Variables|Default|GetbTextDisplayed)
    (Variables|Default|SetSubtitles "")
    (Variables|Default|SetbTextDisplayed false)
    (else
      (HUD|DrawText (Variables|Default|GetSubtitles) (Math|Conversions|ToLinearColor(Color) (Variables|Default|GetTextColor)) (Math|Conversions|ToFloat(Integer) (/ SizeX 5)) (Math|Conversions|ToFloat(Integer) (+ (/ SizeY 2) 200)) (Variables|Default|GetHUDFont) (Variables|Default|GetTextScale) false)
      (Utilities|FlowControl|Delay (Variables|Default|GetDelayTimer))
      (Variables|Default|SetbTextDisplayed true)
      (Variables|Default|SetDelayTimer 3.0))))

(fn ConstructionScript)