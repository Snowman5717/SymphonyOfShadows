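; BP_PhysicsBox is a physics crate interactable that plays collision sounds at the impact point when hit.
; The Hit event picks the heavy crate sound when Z velocity exceeds a threshold, otherwise the regular one, with volume clamped from that velocity.
; Each sound has its own DoOnce gate, reset after a short delay to limit repeats.
; Every hit also prints its normal impulse.
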(event EventActorBeginOverlap
  (params (OtherActor :type Actor%20Object%20Reference)))

(event EventTick
  (params (DeltaSeconds :type Float%20%28single-precision%29)))

(event Collision|EventHit
  (params (MyComp :type Primitive%20Component%20Object%20Reference) (Other :type Actor%20Object%20Reference) (OtherComp :type Primitive%20Component%20Object%20Reference) (bSelfMoved :type Boolean) (HitLocation :type Vector) (HitNormal :type Vector :default "0, 0, 0") (NormalImpulse :type Vector) (Hit :type Hit%20Result%20Structure%20%28by%20ref%29))
  (bind _returnvalue (Transformation|GetVelocity))
  (bind _z (Math|Vector|BreakVector _returnvalue))
  (bind _returnvalue_2 (Math|Conversions|ToVector(Float) _z))
  (bind _returnvalue_3 (Math|Vector|VectorLength _returnvalue_2))
  (bind _returnvalue_4 (Math|Float|Clamp(Float) _returnvalue_3 0.0 1.0))
  (Development|PrintString (Utilities|String|ToString(Vector) NormalImpulse))
  (if (> _z 3e+02)
    (Utilities|FlowControl|DoOnce false :!label _label
      (:Completed
        (Audio|PlaySoundatLocation "/Game/Sounds/Interactables/Crate/CrateHeavyCollision.CrateHeavyCollision" HitLocation "0, 0, 0" _returnvalue_4)
        (Utilities|FlowControl|Delay 0.5)
        (goto _label Reset)))
    (else
      (Utilities|FlowControl|DoOnce false :!label _label_2
        (:Completed
          (Audio|PlaySoundatLocation "/Game/Sounds/Interactables/Crate/CrateCollision.CrateCollision" HitLocation "0, 0, 0" _returnvalue_4)
          (Utilities|FlowControl|Delay 0.4)
          (goto _label_2 Reset))))))

(event EventBeginPlay)

(fn ConstructionScript)